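; Dragon projectile that leaves a breath trigger box where it hits.
; On BeginPlay its Sphere starts with physics-only collision, then enables query and physics collision after a short delay.
; When the Sphere registers a hit, it spawns BP_BreathTriggerBox at the Sphere's location and rotation, scaled up on X and Z, then destroys itself.
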(event OnComponentHit(Sphere)
  (params (HitComponent :type Primitive%20Component%20Object%20Reference) (OtherActor :type Actor%20Object%20Reference) (OtherComp :type Primitive%20Component%20Object%20Reference) (NormalImpulse :type Vector :default "0, 0, 0") (Hit :type Hit%20Result%20Structure%20%28by%20ref%29))
  (bind _sphere (Variables|Default|GetSphere))
  (bind _returnvalue (Transformation|GetWorldTransform _sphere))
  (bind (_location _rotation) (Math|Transform|BreakTransform _returnvalue))
  (Game|SpawnActorfromClass "/Game/DragonNPC/BP_BreathTriggerBox.BP_BreathTriggerBox_C" (Math|Transform|MakeTransform _location _rotation "3.000000,1.000000,3.000000") "Undefined" "MultiplyWithRoot" 0 0)
  (Actor|DestroyActor))

(event EventBeginPlay
  (Collision|SetCollisionEnabled (Variables|Default|GetSphere) "PhysicsOnly")
  (|CallParentFunction)
  (Utilities|FlowControl|Delay 0.4)
  (Collision|SetCollisionEnabled (Variables|Default|GetSphere) "QueryAndPhysics"))

(event Collision|EventActorBeginOverlap
  (params (OtherActor :type Actor%20Object%20Reference))
  (|CallParentFunction OtherActor) ; This node is disabled and will not be called.\nDrag off pins to build functionality.
)

(event EventTick
  (params (DeltaSeconds :type Float%20%28single-precision%29))
  (|CallParentFunction DeltaSeconds) ; This node is disabled and will not be called.\nDrag off pins to build functionality.
)

(fn ConstructionScript
  (|CallParentFunction))