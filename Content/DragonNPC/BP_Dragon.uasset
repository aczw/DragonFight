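; Flying dragon NPC that steers toward a TargetLocation and hurts the player on contact.
; While alive, Tick eases rotation toward the target with RInterpTo and adds forward movement input; once dead, it calls OnDragonDeath.
; Overlapping the player starts a looping timer that drains their health component until an overlap ends.
; AI perception only records SeesPlayer and prints debug messages.
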(event OnTargetPerceptionUpdated(AIPerception)
  (params (Actor :type Actor%20Object%20Reference) (Stimulus :type AI%20Stimulus%20Structure))
  (bind _bsuccessfullysensed (Utilities|Struct|BreakAIStimulus Stimulus))
  (Variables|Default|SetSeesPlayer _bsuccessfullysensed)
  (if _bsuccessfullysensed
    (Development|PrintString "Dragon Sees You")
    (else
      (Development|PrintString "Dragon Loses Sight"))))

(event EventBeginPlay
  (Pawn|Components|CharacterMovement|SetMovementMode (Variables|Character|GetCharacterMovement) "MOVE_Flying" 0))

(event EventTick
  (params (DeltaSeconds :type Float%20%28single-precision%29))
  (bind _returnvalue (Transformation|GetActorLocation))
  (bind _returnvalue_2 (Transformation|GetActorRotation))
  (bind _turnrate (Variables|Default|GetTurnRate))
  (bind _targetlocation (Variables|Default|GetTargetLocation))
  (bind _returnvalue_3 (- _targetlocation _returnvalue))
  (bind _returnvalue_4 (Math|Vector|Normalize _returnvalue_3))
  (bind _returnvalue_5 (Math|Rotator|MakeRotfromX _returnvalue_4))
  (bind _returnvalue_6 (Math|Interpolation|RInterpTo _returnvalue_2 _returnvalue_5 DeltaSeconds _turnrate))
  (bind _isalive (Default|IsAlive (Variables|Default|GetBPC_HealthSystem)))
  (if _isalive
    (for _array_element (Collision|GetOverlappingActors (Variables|Default|GetMawDamage) 0 :!class /Script/Engine.PrimitiveComponent)
      _)
    (switch Utilities|FlowControl|Switch|SwitchonEMovementMode (Variables|/Script/Engine.CharacterMovementComponent|GetMovementMode (Variables|Character|GetCharacterMovement))
      (:MOVE_Flying
        ;[0.15 0.15 0.15 0.5] PD Controller Flight
        (Transformation|SetActorRotation _returnvalue_6)
        (Pawn|Input|AddMovementInput (Math|Rotator|GetRotationXVector _returnvalue_6) (Variables|Default|GetFlightSpeed) false)))
    (else
      (Default|CallOnDragonDeath))))

(event Collision|EventActorBeginOverlap
  (params (OtherActor :type Actor%20Object%20Reference))
  (Utilities|Casting|CastToBP_ThirdPersonCharacter OtherActor)
  (bind _returnvalue (Utilities|Time|SetTimerbyFunctionName 0 "DamagePlayer" 0.3 true))
  (Variables|Default|SetDamageTimer _returnvalue))

(event Collision|EventActorEndOverlap
  (params (OtherActor :type Actor%20Object%20Reference))
  (Utilities|Time|ClearandInvalidateTimerbyHandle (Variables|Default|GetDamageTimer)))

(fn ConstructionScript)

(fn DamagePlayer
  (bind _asbp_third_person_character (Utilities|Casting|CastToBP_ThirdPersonCharacter (Game|Player|GetPlayerPawn 0)))
  (Default|DecreaseHealth (Variables|/Game/ThirdPerson/Blueprints/BP_ThirdPersonCharacter.BP_ThirdPersonCharacter_C|GetBPC_HealthSystem _asbp_third_person_character) 20)
  (Development|PrintString "damaged"))