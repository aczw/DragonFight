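; BP_BreathTriggerBox is a short-lived damage volume, named for the dragon NPC's breath attack, that hurts the player while inside it.
; Shortly after spawning it checks for an already-overlapping third-person character, and begin overlap also starts a looping timer that repeatedly calls DamagePlayer.
; DamagePlayer applies damage to player pawn 0 through AttemptToTakeDamage.
; Any actor ending overlap clears the timer, and the box destroys itself after ten seconds.
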(event EventBeginPlay
  (Utilities|FlowControl|Delay 0.1)
  (for _array_element (Collision|GetOverlappingActors 0 :!class /Script/Engine.Actor)
    (Utilities|Casting|CastToBP_ThirdPersonCharacter _array_element)
    (bind _returnvalue (Utilities|Time|SetTimerbyFunctionName 0 "DamagePlayer" 0.3 true))
    (Variables|Default|SetDamageTimer _returnvalue))
  (Utilities|FlowControl|Delay 1e+01)
  (Actor|DestroyActor))

(event Collision|EventActorBeginOverlap
  (params (OtherActor :type Actor%20Object%20Reference))
  (Utilities|Casting|CastToBP_ThirdPersonCharacter OtherActor)
  (bind _returnvalue (Utilities|Time|SetTimerbyFunctionName 0 "DamagePlayer" 0.3 true))
  (Variables|Default|SetDamageTimer _returnvalue))

(event Collision|EventActorEndOverlap
  (params (OtherActor :type Actor%20Object%20Reference))
  (Utilities|Time|ClearandInvalidateTimerbyHandle (Variables|Default|GetDamageTimer)))

(fn ConstructionScript)

(fn DamagePlayer
  (bind _asbp_third_person_character (Utilities|Casting|CastToBP_ThirdPersonCharacter (Game|Player|GetPlayerPawn 0)))
  (Default|AttempttoTakeDamage _asbp_third_person_character 5))