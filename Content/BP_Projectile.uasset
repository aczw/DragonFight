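; BP_Projectile is a projectile that damages dragon enemies on impact.
; On BeginPlay it launches its physics sphere forward with a single impulse and sets it to ignore its PlayerParent while moving.
; When the sphere hits something, it lowers the health of a hit BP_Dragon through its BPCHealthSystem component, then destroys itself whatever it struck.
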(event OnComponentHit(Sphere)
  (params (HitComponent :type Primitive%20Component%20Object%20Reference) (OtherActor :type Actor%20Object%20Reference) (OtherComp :type Primitive%20Component%20Object%20Reference) (NormalImpulse :type Vector :default "0, 0, 0") (Hit :type Hit%20Result%20Structure%20%28by%20ref%29))
  (Collision|IgnoreActorwhenMoving (Variables|Default|GetSphere) (Variables|Default|GetPlayer%20Parent) true)
  (bind _asbp_dragon (Utilities|Casting|CastToBP_Dragon OtherActor)
    (:then
      (Default|DecreaseHealth (Variables|/Game/DragonNPC/BP_Dragon.BP_Dragon_C|GetBPC_HealthSystem _asbp_dragon) 5)
      (Actor|DestroyActor))
    (:CastFailed
      (Actor|DestroyActor))))

(event EventBeginPlay
  (Collision|IgnoreActorwhenMoving (Variables|Default|GetSphere) (Variables|Default|GetPlayer%20Parent) true)
  (Physics|AddImpulse (Variables|Default|GetSphere) (* (Variables|Default|GetForward) "2000.000000,2000.000000,2000.000000") "None" false)
  (Collision|IgnoreActorwhenMoving (Variables|Default|GetSphere) (Variables|Default|GetPlayer%20Parent) true))

(event Collision|EventActorBeginOverlap
  (params (OtherActor :type Actor%20Object%20Reference)))

(event EventTick
  (params (DeltaSeconds :type Float%20%28single-precision%29)))

(fn ConstructionScript)