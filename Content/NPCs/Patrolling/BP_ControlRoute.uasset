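; BP_ControlRoute is a patrol route actor that serves spline points as waypoints, one at a time.
; GetPointLocation returns the world location of the PatrolRoute spline point at the current index.
; IncrementSplineIndex steps the index by a direction value and reverses that direction at either end of the spline, giving a back-and-forth path, with a debug print at each reversal.
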(event EventBeginPlay)

(event Collision|EventActorBeginOverlap
  (params (OtherActor :type Actor%20Object%20Reference)))

(event EventTick
  (params (DeltaSeconds :type Float%20%28single-precision%29)))

(fn ConstructionScript)

(fn GetPointLocation
  (return (Spline|GetLocationatSplinePoint (Variables|Default|GetPatrol%20Route) (Variables|Default|GetSplitPointIdx) "World")))

(fn IncrementSplineIndex
  (bind _output_get (Variables|Default|SetSplitPointIdx (+ (Variables|Default|GetSplitPointIdx) (Variables|Default|GetDirection))))
  (if (or (<= _output_get 0) (>= _output_get (- (Spline|GetNumberOfSplinePoints (Variables|Default|GetPatrol%20Route)) 1)))
    (Development|PrintString "BRANCH END TRUE")
    (Variables|Default|SetDirection (* (Variables|Default|GetDirection) -1))))