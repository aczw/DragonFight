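; Base enemy NPC Blueprint that passes AI perception updates to its controller's Blackboard.
; Any target perception update sets SeesPlayer to true, without checking the stimulus or actor, and nothing here clears it.
; It then casts its controller to AIC_Enemy_Base and writes that boolean as a byte into the state enum key.
; Debug prints report the change; other events and construction add no logic.
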(event OnTargetPerceptionUpdated(AIPerception)
  (params (Actor :type Actor%20Object%20Reference) (Stimulus :type AI%20Stimulus%20Structure))
  (bind _output_get (Variables|Default|SetSees%20Player true))
  (bind _asaic_enemy_base (Utilities|Casting|CastToAIC_Enemy_Base (Pawn|GetController)))
  (AI|Components|Blackboard|SetValueasEnum (AI|GetBlackboard _asaic_enemy_base) (Variables|/Game/NPCs/AIC_Enemy_Base.AIC_Enemy_Base_C|GetState%20Key%20Name _asaic_enemy_base) (Math|Conversions|ToByte(Integer) _output_get))
  (Development|PrintString "STATE ACTIVATED")
  (Development|PrintString (Utilities|String|ToString(Byte) (Math|Conversions|ToByte(Integer) _output_get))))

(event EventBeginPlay)

(event Collision|EventActorBeginOverlap
  (params (OtherActor :type Actor%20Object%20Reference)))

(event EventTick
  (params (DeltaSeconds :type Float%20%28single-precision%29)))

(fn ConstructionScript
  (|CallParentFunction))