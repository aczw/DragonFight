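; BPC_HealthSystem is a health component that tracks damage, healing and death for its owning actor, either the third-person character or the dragon.
; DecreaseHealth floors Health at zero and, on death, casts the owner to trigger OnDeathMessage on the character or CallOnDragonDeath on the dragon, with debug prints.
; IncreaseHealth adds without an upper limit, IsAlive checks for positive health, and ResetHealth restores a fixed value.
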(event EventBeginPlay)

(event EventTick
  (params (DeltaSeconds :type Float%20%28single-precision%29)))

(fn DecreaseHealth
  (params (Amount :type Integer))
  (bind _returnvalue (Components|GetOwner))
  (bind _output_get (Variables|Default|SetHealth (Math|Integer|Max(Integer) (- (Variables|Default|GetHealth) Amount))))
  (Development|PrintString (Utilities|String|Append "[Debug] Health now " (Utilities|String|ToString(Integer) _output_get)))
  (if (== (Math|Integer|Max(Integer) (- (Variables|Default|GetHealth) Amount)) 0)
    (bind _asbp_third_person_character (Utilities|Casting|CastToBP_ThirdPersonCharacter _returnvalue)
      (:then
        (Development|PrintString "[Debug] Casted on death")
        (Class|BPICharacterInterface|OnDeath(Message) _asbp_third_person_character))
      (:CastFailed
        (bind _asbp_dragon (Utilities|Casting|CastToBP_Dragon _returnvalue))
        (Default|CallOnDragonDeath _asbp_dragon)
        (Development|PrintString "[Debug] Event Called")))))

(fn IncreaseHealth
  (params (Amount :type Integer))
  (Variables|Default|SetHealth (+ (Variables|Default|GetHealth) Amount)))

(fn IsAlive
  (return (> (Variables|Default|GetHealth) 0)))

(fn ResetHealth
  (Variables|Default|SetHealth 100))